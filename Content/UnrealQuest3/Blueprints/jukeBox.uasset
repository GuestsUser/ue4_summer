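; Jukebox actor that cycles through three sounds when the player presses S while standing in its hit area.
; HitArea overlap events set a flag for actors tagged "player", and all sounds are stopped at BeginPlay.
; Tick polls the S key, using a hold counter to react only on the initial press.
; Each press advances a modulo-3 index, playing the matching audio component and stopping the other two.
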(event OnComponentBeginOverlap(HitArea)
  (params (OverlappedComponent :type Primitive%20Component%20Object%20Reference) (OtherActor :type Actor%20Object%20Reference) (OtherComp :type Primitive%20Component%20Object%20Reference) (OtherBodyIndex :type Integer) (bFromSweep :type Boolean) (SweepResult :type Hit%20Result%20Structure%20%28by%20ref%29))
  (if (Actor|ActorHasTag OtherActor "player")
    ;[1 1 1] playerが接触してた時だけ設定する
    (Variables|Default|Setplayer_overrap true)))

(event OnComponentEndOverlap(HitArea)
  (params (OverlappedComponent :type Primitive%20Component%20Object%20Reference) (OtherActor :type Actor%20Object%20Reference) (OtherComp :type Primitive%20Component%20Object%20Reference) (OtherBodyIndex :type Integer))
  (if (Actor|ActorHasTag OtherActor "player")
    ;[1 1 1] playerが接触してた時だけ設定する
    (Variables|Default|Setplayer_overrap false)))

(event EventBeginPlay
  (Audio|Components|Audio|Stop (Variables|Default|Getsound0))
  (Audio|Components|Audio|Stop (Variables|Default|Getsound1))
  (Audio|Components|Audio|Stop (Variables|Default|Getsound2)))

(event Collision|EventActorBeginOverlap
  (params (OtherActor :type Actor%20Object%20Reference)))

(event EventTick
  (params (DeltaSeconds :type Float%20%28single-precision%29))
  (bind _sound0 (Variables|Default|Getsound0))
  (bind _sound1 (Variables|Default|Getsound1))
  (bind _sound2 (Variables|Default|Getsound2))
  (if (and (Variables|Default|Getplayer_overrap) (== (Class|PlayerController|GetInputAnalogKeyState (Game|GetPlayerController 0) "S") 1.0))
    ;[1 1 1] 押しっぱなしを検知してしまうのでそれの回避用
    ;;[1 1 1] ボタン入力検知でcountに1加算
    (Variables|Default|Sethold_count (+ (Variables|Default|Gethold_count) 1))
    (if (<= (Variables|Default|Gethold_count) 1)
      (Variables|Default|Setcount (Math|Integer|%(Integer) (+ (Variables|Default|Getcount) 1) 3))
      (if (== (Variables|Default|Getcount) 0)
        (Audio|Components|Audio|Play _sound0 0.0)
        (else
          (Audio|Components|Audio|Stop _sound0)))
      (if (== (Variables|Default|Getcount) 1)
        (Audio|Components|Audio|Play _sound1 0.0)
        (else
          (Audio|Components|Audio|Stop _sound1)))
      (if (== (Variables|Default|Getcount) 2)
        (Audio|Components|Audio|Play _sound2 0.0)
        (else
          (Audio|Components|Audio|Stop _sound2))))
    (else
      ;;[1 1 1] 入力が切れたら0にする
      (Variables|Default|Sethold_count 0))))

(fn ConstructionScript)