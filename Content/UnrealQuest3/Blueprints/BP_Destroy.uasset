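; BP_Destroy is a destructible object that shatters when hit by an actor tagged "bullet", then fades out and destroys itself.
; The hit halves the actor's scale, applies radius damage to the Destructible component and starts a timeline that counts up to a delay limit.
; Tick then drives FadeOut, lowering the color alpha on a dynamic material created at BeginPlay until the actor is destroyed.
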(event OnComponentHit(Destructible)
  (params (HitComponent :type Primitive%20Component%20Object%20Reference) (OtherActor :type Actor%20Object%20Reference) (OtherComp :type Primitive%20Component%20Object%20Reference) (NormalImpulse :type Vector :default "0, 0, 0") (Hit :type Hit%20Result%20Structure%20%28by%20ref%29))
  (bind _destructible (Variables|Default|GetDestructible))
  (if (Actor|ActorHasTag OtherActor "bullet")
    (Transformation|SetActorScale3D "0.500000,0.500000,0.500000")
    (Class|DestructibleComponent|ApplyRadiusDamage _destructible 1e+02 (Transformation|GetWorldLocation _destructible) 1e+02 1e+03 false)
    (Timeline|del_count Play
      (:Update
        (Variables|Default|Setcount (+ (Variables|Default|Getcount) (Variables|Default|Getdelta_time)))
        (if (> (Variables|Default|Getcount) (Variables|Default|Getdel_limit))
          (Variables|Default|Setfade_run true)
          (CallFunction|FadeOut)
          (Timeline|del_count Stop))))))

(event EventBeginPlay
  (bind _returnvalue (Rendering|Material|CreateDynamicMaterialInstance "/Game/UnrealQuest3/Materials/CubeMaterial.CubeMaterial" "None" "None" :!class /Script/Engine.KismetMaterialLibrary))
  (bind _output_get (Variables|Default|Setmaterial _returnvalue))
  (Rendering|Material|SetMaterial (Variables|Default|GetDestructible) 0 _output_get))

(event Collision|EventActorBeginOverlap
  (params (OtherActor :type Actor%20Object%20Reference)))

(event EventTick
  (params (DeltaSeconds :type Float%20%28single-precision%29))
  (Variables|Default|Setdelta_time DeltaSeconds)
  (if (Variables|Default|Getfade_run)
    (CallFunction|FadeOut)))

(fn ConstructionScript)

(fn FadeOut
  (bind _output_get (Variables|Default|Setfade_count (+ (Variables|Default|Getdelta_time) (Variables|Default|Getfade_count))))
  (bind _output_get_2 (LocalVariables|Setalpha (- 1.0 (/ _output_get (Variables|Default|Getfade_limit)))))
  (if (< _output_get_2 0.0)
    (Variables|Default|Setfade_run false)
    (Actor|DestroyActor)
    (else
      (Rendering|Material|SetVectorParameterValue (Variables|Default|Getmaterial) "color" (Utilities|Struct|MakeLinearColor 1.0 1.0 1.0 _output_get_2) :!class /Script/Engine.MaterialInstanceDynamic))))