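; BP_Throw is a thrown ball projectile gimmick that launches like a pitch when spawned.
; BeginPlay enables physics on its collision component and sets the velocity to a LaunchVector.
; Hitting anything not tagged player hides the sphere and flags it for deletion.
; Tick destroys the actor one frame later, so other objects such as cubes still receive the hit without a visible bounce.
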(event OnComponentHit(Collision)
  (params (HitComponent :type Primitive%20Component%20Object%20Reference) (OtherActor :type Actor%20Object%20Reference) (OtherComp :type Primitive%20Component%20Object%20Reference) (NormalImpulse :type Vector :default "0, 0, 0") (Hit :type Hit%20Result%20Structure%20%28by%20ref%29))
  ;[1 1 1] 何れかのオブジェクトと接触で削除
  ;;[1 1 1] 接触がプレイヤーだった場合消さない
  (if (not (Actor|ActorHasTag OtherActor "player"))
    ;;[1 1 1] すぐ消さないが消えないとバウンドするので非表示化
    (Variables|Default|Setdel true)
    (Development|SetHiddeninGame (Variables|Default|GetSphere) true true)))

(event EventTick
  (params (DeltaSeconds :type Float%20%28single-precision%29))
  ;[1 1 1] cube等にヒット判定を伝える為、当たってもすぐ消さず、1フレーム待つ
  (if (Variables|Default|Getdel)
    (if (> (Variables|Default|Getcount) 0)
      (Actor|DestroyActor)
      (else
        (Variables|Default|Setcount 1)))))

(event EventBeginPlay
  (bind _collision (Variables|Default|GetCollision))
  ;[1 1 1] Spawn時にボールを投げるイメージで飛ばす処理
  (Physics|SetSimulatePhysics _collision true)
  (Class|PrimitiveComponent|SetAllPhysicsLinearVelocity _collision (Variables|Default|GetLaunchVector) false))

(fn ConstructionScript)