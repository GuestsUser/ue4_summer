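; MoveCube is an actor that moves along a timeline-driven offset from its starting location until a bullet stops it.
; While enabled, Tick sets the timeline play rate from Time and plays it, with the curve output scaling Range for each teleported position.
; A mesh hit from an actor tagged "bullet" clears Enable, so Tick stops the timeline.
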(event OnComponentHit(StaticMeshComponent)
  (params (HitComponent :type Primitive%20Component%20Object%20Reference) (OtherActor :type Actor%20Object%20Reference) (OtherComp :type Primitive%20Component%20Object%20Reference) (NormalImpulse :type Vector :default "0, 0, 0") (Hit :type Hit%20Result%20Structure%20%28by%20ref%29))
  (if (Actor|ActorHasTag OtherActor "bullet")
    (Variables|Default|Setenable false)))

(event EventBeginPlay
  (Variables|Default|SetiniPos (Transformation|GetActorLocation)))

(event Collision|EventActorBeginOverlap
  (params (OtherActor :type Actor%20Object%20Reference)))

(event EventTick
  (params (DeltaSeconds :type Float%20%28single-precision%29))
  (if (Variables|Default|Getenable)
    (Components|Timeline|SetPlayRate (Variables|Default|Getタイムライン_0) (/ 1.0 (Variables|Default|Gettime)))
    (bind __1_1 (Timeline|タイムライン_0 Play)
      (:Update
        (Transformation|SetActorLocation (+ (* (Variables|Default|Getrange) __1_1) (Variables|Default|GetiniPos)) false true)))
    (else
      (Timeline|タイムライン_0 Stop))))

(fn ConstructionScript)